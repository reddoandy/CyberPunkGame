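; Game instance that handles post-login flow and session hand-off between lobby and matches.
; On server login it creates a dedicated Advanced Sessions lobby on LobbyMap, otherwise asks BP_BattleGameMode to create a battle session; player login shows the lobby-choice widget.
; Events move players by destroying and joining a session, or joining a match port after a delay; match-found results are only printed.
; Several unwired chains hold older login, session-search and travel experiments.
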(event Custom|CustomEvent
  (bind _returnvalue (Game|GetPlayerController 0))
  (bind _asmy_player_controller (Utilities|Casting|CastToMyPlayerController _returnvalue))
  (bind _returnvalue_2 (UserInterface|CreateWidget "/Game/Blueprints/UI/ChooseLobby_UI.ChooseLobby_UI_C" (Class|GameplayStatics|GetPlayerControllerfromID (Class|GameplayStatics|GetPlayerControllerID _returnvalue))))
  (UserInterface|Viewport|AddtoViewport _returnvalue_2 0)
  (Development|PrintString "login"))

(event Custom|DestoryAndJoin
  (params (Result :type Blueprint%20Session%20Result%20Structure))
  (bind _returnvalue (Game|GetPlayerController 0))
  (|DestroySession _returnvalue
    (:OnSuccess
      (Development|PrintString (Class|AdvancedSessionsLibrary|GetSessionIDasString Result))
      (|JoinSession _returnvalue Result
        (:OnSuccess
          (Development|PrintString "Join Match"))
        (:OnFailure
          (Development|PrintString "Fail"))))))

(event EventInit
  (Utilities|FlowControl|Delay 2.0))

(event EventServerCompleteLogin
  (bind _returnvalue (Game|GetCurrentLevelName true))
  (Development|PrintString _returnvalue)
  (if (Utilities|Enum|Equal(Enum) _returnvalue "LobbyMap")
    (|AdvancedSession (Utilities|Array|MakeArray (Class|AdvancedSessionsLibrary|MakeLiteralSessionPropertyString "Name" "Lobby1") (Class|AdvancedSessionsLibrary|MakeLiteralSessionPropertyString "Type" "Lobby")) (Game|GetPlayerController 0) 100 0 false true true true false true false false false true false true
      (:OnSuccess
        (Development|PrintString "Hello")))
    (else
      (Default|CreateBattleSession (.AsBP%20Battle%20Game%20Mode (Utilities|Casting|CastToBP_BattleGameMode (Game|GetGameMode)))))))

(event EventSendMatchFoundResult
  (params (Result :type Match%20Result%20Structure%20%28by%20ref%29))
  (Development|PrintString (Utilities|String|ToString(Boolean) (.ismatched Result)))
  (Development|PrintString (.matchid Result))
  (for _array_element (.players Result)
    (Development|PrintString _array_element)))

(event EventPlayerCompleteLogin
  (bind _returnvalue (Game|GetPlayerController 0))
  (bind _asmy_player_controller (Utilities|Casting|CastToMyPlayerController _returnvalue))
  (bind _returnvalue_2 (UserInterface|CreateWidget "/Game/Blueprints/UI/ChooseLobby_UI.ChooseLobby_UI_C" (Class|GameplayStatics|GetPlayerControllerfromID (Class|GameplayStatics|GetPlayerControllerID _returnvalue))))
  (UserInterface|Viewport|AddtoViewport _returnvalue_2 0)
  (Development|PrintString "login"))

(event EventReadytoJoinMatchEvent
  (params (MatchPort :type Integer%20%28by%20ref%29))
  (Utilities|FlowControl|Delay 5.0)
  (Class|MyGameInstance|MyJoinMatch (Game|GetPlayerController 0) MatchPort)
  (Development|PrintString (Utilities|String|ToString(Integer) MatchPort)))