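; Battle game mode that creates a dedicated-server session tagged with a match ID and runs team character selection and spawning.
; Players register into Red or Blue arrays; reaching MaxPlayer starts character choice on each PreGameChar and the GameState's pre-game countdown.
; GetSpawnPoint indexes PlayerStarts by numeric tag, then spawns and possesses each controller's SelectChar.
; Blue uses start indices from zero, Red from MaxPlayer/2.
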(event Custom|CreateBattleSession
  (bind _matchid (Variables|Default|GetMatchId))
  (Class|BattleGameModeBase|GetMatchId)
  (Development|PrintString _matchid)
  (|AdvancedSession (Utilities|Array|MakeArray (Class|AdvancedSessionsLibrary|MakeLiteralSessionPropertyString "MatchId" _matchid)) (Game|GetPlayerController 0) 100 0 false true true true false true false false false true false true
    (:OnSuccess
      (Class|BattleGameModeBase|SessionReady))))

(event Custom|InputPlayerInfo
  (params (PlayerController :type Player%20Controller%20Object%20Reference%20%28by%20ref%29) (Team :type String) (index :type Integer))
  (bind _redteamplayer (Variables|Default|GetRedTeamPlayer))
  (bind _blueteamplayer (Variables|Default|GetBlueTeamPlayer))
  (Utilities|Array|SetArrayElem (select (Utilities|Enum|Equal(Enum) Team "RedTeam") _redteamplayer _blueteamplayer) index PlayerController true)
  (if (>= (+ (Utilities|Array|Length _blueteamplayer) (Utilities|Array|Length _redteamplayer)) (Variables|Default|GetMaxPlayer))
    (CallFunction|ChooseCharacter)
    (Development|PrintString "Hello Choose")))

(event Custom|ChooseCharacter
  (bind _array_element (Utilities|Array|ForEachLoopwithBreak (Variables|Default|GetRedTeamPlayer))
    (:LoopBody
      (Default|Choosecharacter (.AsPre%20Game%20Char (Utilities|Casting|CastToPreGameChar (Pawn|GetControlledPawn _array_element)))))
    (:Completed
      (bind _array_element_2 (Utilities|Array|ForEachLoopwithBreak (Variables|Default|GetBlueTeamPlayer))
        (:LoopBody
          (Default|Choosecharacter (.AsPre%20Game%20Char (Utilities|Casting|CastToPreGameChar (Pawn|GetControlledPawn _array_element_2)))))
        (:Completed
          (Default|PreGameCountDown (.AsBattle%20Game%20State%20Base (Utilities|Casting|CastToBattleGameStateBase (Game|GetGameState))))
          (Development|PrintString "Hello Count"))))))

(event Custom|SpawnChooseChar
  (bind _startpoint (Variables|Default|GetStartPoint))
  (bind (_array_element _array_index) (Utilities|Array|ForEachLoopwithBreak (Variables|Default|GetRedTeamPlayer))
    (:LoopBody
      (bind _returnvalue (Game|SpawnActorfromClass (Variables|/Game/Blueprints/MainChar/MyPlayerController.MyPlayerController_C|GetSelectChar (.AsMy%20Player%20Controller (Utilities|Casting|CastToMyPlayerController _array_element))) (Transformation|GetActorTransform (Utilities|Array|Get(acopy) _startpoint (+ _array_index (/ (Variables|Default|GetMaxPlayer) 2)))) "Undefined" "MultiplyWithRoot" (.AsMy%20Player%20Controller (Utilities|Casting|CastToMyPlayerController _array_element)) 0))
      (Default|EndChoosing (.AsPre%20Game%20Char (Utilities|Casting|CastToPreGameChar (Pawn|GetControlledPawn _array_element))))
      (Pawn|Possess (.AsMy%20Player%20Controller (Utilities|Casting|CastToMyPlayerController _array_element)) _returnvalue))
    (:Completed
      (bind (_array_element_2 _array_index_2) (Utilities|Array|ForEachLoopwithBreak (Variables|Default|GetBlueTeamPlayer))
        (:LoopBody
          (bind _returnvalue_2 (Game|SpawnActorfromClass (Variables|/Game/Blueprints/MainChar/MyPlayerController.MyPlayerController_C|GetSelectChar (.AsMy%20Player%20Controller (Utilities|Casting|CastToMyPlayerController _array_element_2))) (Transformation|GetActorTransform (Utilities|Array|Get(acopy) _startpoint _array_index_2)) "Undefined" "MultiplyWithRoot" (.AsMy%20Player%20Controller (Utilities|Casting|CastToMyPlayerController _array_element_2)) 0))
          (Default|EndChoosing (.AsPre%20Game%20Char (Utilities|Casting|CastToPreGameChar (Pawn|GetControlledPawn _array_element_2))))
          (Pawn|Possess (.AsMy%20Player%20Controller (Utilities|Casting|CastToMyPlayerController _array_element_2)) _returnvalue_2))))))

(event Custom|GetSpawnPoint
  (bind _outactors (Actor|GetAllActorsOfClass "/Script/Engine.PlayerStart"))
  (for _array_element _outactors
    (Utilities|Array|SetArrayElem (Variables|Default|GetStartPoint) (Math|Conversions|ToInteger(Byte) (Utilities|String|ToString(Name) (Variables|/Script/Engine.PlayerStart|GetPlayerStartTag _array_element))) _array_element))
  (CallFunction|SpawnChooseChar))

(event EventBeginPlay)

(event EventTick
  (params (DeltaSeconds :type Float%20%28single-precision%29)))

(fn ConstructionScript)