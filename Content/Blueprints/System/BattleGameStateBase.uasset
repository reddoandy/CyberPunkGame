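; Battle game state that simulates bullets on the server and runs the pre-game countdown.
; Each tick it steps every registered bullet struct by velocity plus gravity, without delta-time scaling, moves its actor and sphere-traces the path.
; A hit destroys the bullet and damages the target only if its TeamComponent team differs from the instigator's.
; When the server-time countdown elapses, the server tells BP_BattleGameMode once to spawn character selection.
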(event Custom|SpawnBulletServer
  (params (Bullet :type S%20Bullet%20Simulation%20Structure))
  (Utilities|Array|Add (Variables|Default|GetBullets) Bullet))

(event Custom|PreGameCountDown
  (Variables|Default|SetStartCountTime (GameState|GetServerWorldTimeSeconds)))

(event Custom|SpawnBullet
  (params (Bullets :type S%20Bullet%20Simulation%20Structure%20%28by%20ref%29))
  (Utilities|Array|Add (Variables|Default|GetBullets) Bullets))

(event EventBeginPlay)

(event EventTick
  (params (DeltaSeconds :type Float%20%28single-precision%29))
  (bind _returnvalue (Networking|IsServer))
  (bind _bullets (Variables|Default|GetBullets))
  (Utilities|FlowControl|Sequence
    (:then_0
      (if _returnvalue
        (bind (_array_element _array_index) (Utilities|Array|ForEachLoopwithBreak _bullets)
          (:LoopBody
            (bind _output_get (Variables|Default|SetOldPos (.Position (Utilities|Struct|BreakS_BulletSimulation _array_element))))
            (Utilities|Array|SetArrayElem _bullets _array_index (Utilities|Struct|MakeS_BulletSimulation (+ (.Position (Utilities|Struct|BreakS_BulletSimulation _array_element)) (+ (.Velocity (Utilities|Struct|BreakS_BulletSimulation _array_element)) (Math|Vector|MakeVector 0.0 0.0 (Variables|Default|GetGravityScale)))) (+ (.Velocity (Utilities|Struct|BreakS_BulletSimulation _array_element)) (Math|Vector|MakeVector 0.0 0.0 (Variables|Default|GetGravityScale))) (.Damage (Utilities|Struct|BreakS_BulletSimulation _array_element)) (.ActorInstigator (Utilities|Struct|BreakS_BulletSimulation _array_element)) (.BulletActor (Utilities|Struct|BreakS_BulletSimulation _array_element))))
            (bind (_outhit _returnvalue_2) (Collision|SphereTraceForObjects _output_get (.Position (Utilities|Struct|BreakS_BulletSimulation _array_element)) 1.0 (Utilities|Array|MakeArray "ObjectTypeQuery1" "ObjectTypeQuery2" "ObjectTypeQuery3" "ObjectTypeQuery4" "ObjectTypeQuery5") false (Utilities|Array|MakeArray (.ActorInstigator (Utilities|Struct|BreakS_BulletSimulation _array_element))) "ForDuration"))
            (Transformation|SetActorLocation (.BulletActor (Utilities|Struct|BreakS_BulletSimulation _array_element)) (.Position (Utilities|Struct|BreakS_BulletSimulation _array_element)) false false)
            (if _returnvalue_2
              (Development|PrintString "Hit")
              (Development|PrintString (Utilities|GetDisplayName (.HitActor (Collision|BreakHitResult _outhit))))
              (Utilities|IsValid (Actor|GetComponentbyClass (.HitActor (Collision|BreakHitResult _outhit)) "/Game/Blueprints/System/TeamComponent.TeamComponent_C")
                (:Is%20Valid
                  (Development|PrintString (Variables|/Game/Blueprints/System/TeamComponent.TeamComponent_C|GetTeam (Actor|GetComponentbyClass (.HitActor (Collision|BreakHitResult _outhit)) "/Game/Blueprints/System/TeamComponent.TeamComponent_C")))
                  (Development|PrintString (Variables|/Game/Blueprints/System/TeamComponent.TeamComponent_C|GetTeam (Actor|GetComponentbyClass (.ActorInstigator (Utilities|Struct|BreakS_BulletSimulation _array_element)) "/Game/Blueprints/System/TeamComponent.TeamComponent_C")))
                  (if (Utilities|Enum|Equal(Enum) (Variables|/Game/Blueprints/System/TeamComponent.TeamComponent_C|GetTeam (Actor|GetComponentbyClass (.HitActor (Collision|BreakHitResult _outhit)) "/Game/Blueprints/System/TeamComponent.TeamComponent_C")) (Variables|/Game/Blueprints/System/TeamComponent.TeamComponent_C|GetTeam (Actor|GetComponentbyClass (.ActorInstigator (Utilities|Struct|BreakS_BulletSimulation _array_element)) "/Game/Blueprints/System/TeamComponent.TeamComponent_C")))
                    _
                    (else
                      (Game|Damage|ApplyDamage (.HitActor (Collision|BreakHitResult _outhit)) (.Damage (Utilities|Struct|BreakS_BulletSimulation _array_element)) 0 0 "/Game/Blueprints/System/DamageType/NormalDamage.NormalDamage_C"))))
                (:Is%20Not%20Valid
                  _))
              (Actor|DestroyActor (.BulletActor (Utilities|Struct|BreakS_BulletSimulation _array_element)))
              (Utilities|Array|RemoveItem _bullets _array_element))))))
    (:then_1
      (if (>= (- (GameState|GetServerWorldTimeSeconds) (Variables|Default|GetStartCountTime)) (Variables|Default|GetCountTime))
        (if _returnvalue
          (Utilities|FlowControl|DoOnce false
            (:Completed
              (Default|SpawnChooseChar (.AsBP%20Battle%20Game%20Mode (Utilities|Casting|CastToBP_BattleGameMode (Game|GetGameMode)))))))))))

(fn ConstructionScript)