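; Main character shooting system that handles firing and reloading, gated by the player state's Normal playing state.
; LMB fires through server-named events at a ShootingSpeed-based rate, or reloads when ammo is empty.
; Firing traces from the camera to aim a TestAmmo actor spawned at the Niagara component, then passes it with velocity and damage to BattleGameStateBase's SpawnBullet.
; Reloading holds the Reloading state for a short delay, then refills ammo.
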(event Custom|Reload_Server
  (bind _ownerchar (Variables|Default|GetOwnerChar))
  (bind _playerstate (Variables|/Script/Engine.Pawn|GetPlayerState _ownerchar))
  (bind _asmy_player_state (Utilities|Casting|CastToMyPlayerState _playerstate))
  (Development|PrintString "reload")
  (Default|ChangePlayingState _asmy_player_state "NewEnumerator3")
  (Utilities|FlowControl|Delay 1.0)
  (Variables|Default|SetAmmo (Variables|Default|GetMaxAmmo))
  (Default|ChangePlayingState _asmy_player_state "NewEnumerator0"))

(event Custom|Fire_Server
  (bind _ownerchar (Variables|Default|GetOwnerChar))
  (bind _ownerchar_2 (Variables|Default|GetOwnerChar))
  (bind _niagara (Variables|/Game/Blueprints/MainChar/DefaultChar.DefaultChar_C|GetNiagara _ownerchar))
  (bind _camera (Variables|/Game/Blueprints/MainChar/DefaultChar.DefaultChar_C|GetCamera _ownerchar_2))
  (bind _returnvalue (Transformation|GetWorldLocation _niagara))
  (bind _returnvalue_2 (Math|Vector|GetForwardVector _camera))
  (bind _returnvalue_3 (Transformation|GetWorldLocation _camera))
  (bind _returnvalue_4 (* _returnvalue_2 1e+04))
  (bind _returnvalue_5 (+ _returnvalue _returnvalue_4))
  (Math|Integer|DecrementInt (Variables|Default|GetAmmo)
    (:%20%20
      (bind (_outhit _returnvalue_6) (Collision|LineTraceByChannel _returnvalue_3 _returnvalue_5 "TraceTypeQuery1" false 0 "ForDuration"))
      (bind _returnvalue_7 (Game|SpawnActorfromClass "/Game/Blueprints/MainChar/TestAmmo.TestAmmo_C" (Math|Transform|MakeTransform _returnvalue (Math|Rotator|FindLookatRotation _returnvalue (Math|Vector|SelectVector (.Location (Collision|BreakHitResult _outhit)) _returnvalue_5 _returnvalue_6)) "1.000000,1.000000,1.000000") "Undefined" "MultiplyWithRoot" 0 (Variables|Default|GetOwnerChar) 0))
      (Default|SpawnBullet (.AsBattle%20Game%20State%20Base (Utilities|Casting|CastToBattleGameStateBase (Game|GetGameState))) (Utilities|Struct|MakeS_BulletSimulation _returnvalue (* (Math|Vector|Normalize (- (Math|Vector|SelectVector (.Location (Collision|BreakHitResult _outhit)) _returnvalue_5 _returnvalue_6) _returnvalue_3)) 5e+02) 1e+01 (Variables|Default|GetOwnerChar) _returnvalue_7)))))

(event Input|EnhancedActionEvents|EnhancedInputActionIA_LMB
  (params (ActionValue :type Boolean) (ElapsedSeconds :type Float%20%28double-precision%29) (TriggeredSeconds :type Float%20%28double-precision%29) (InputAction :type Input%20Action%20Object%20Reference :default "/Game/Blueprints/Input/Actions/IA_LMB.IA_LMB"))
  (switch Utilities|FlowControl|Switch|SwitchonPlayingState (Variables|/Game/Blueprints/MainChar/MyPlayerState.MyPlayerState_C|GetPlayingState (.AsMy%20Player%20State (Utilities|Casting|CastToMyPlayerState (Variables|/Script/Engine.Pawn|GetPlayerState (Variables|Default|GetOwnerChar)))))
    (:NewEnumerator0
      (if (> (Variables|Default|GetAmmo) 0)
        (Utilities|FlowControl|DoOnce false :!label _label
          (:Completed
            (Utilities|FlowControl|Sequence
              (:then_0
                (CallFunction|FireServer))
              (:then_1
                (Utilities|FlowControl|Delay (/ 1.0 (Variables|Default|GetShootingSpeed)))
                (goto _label Reset)))))
        (else
          (CallFunction|ReloadServer))))))

(event Input|EnhancedActionEvents|EnhancedInputActionIA_Reload
  (params (ActionValue :type Boolean) (ElapsedSeconds :type Float%20%28double-precision%29) (TriggeredSeconds :type Float%20%28double-precision%29) (InputAction :type Input%20Action%20Object%20Reference :default "/Game/Blueprints/Input/Actions/IA_Reload.IA_Reload"))
  (switch Utilities|FlowControl|Switch|SwitchonPlayingState (Variables|/Game/Blueprints/MainChar/MyPlayerState.MyPlayerState_C|GetPlayingState (.AsMy%20Player%20State (Utilities|Casting|CastToMyPlayerState (Variables|/Script/Engine.Pawn|GetPlayerState (Variables|Default|GetOwnerChar)))))
    (:NewEnumerator0
      (if (!= (Variables|Default|GetAmmo) (Variables|Default|GetMaxAmmo))
        (CallFunction|ReloadServer)))))

(event EventBeginPlay)

(event EventTick
  (params (DeltaSeconds :type Float%20%28single-precision%29)))