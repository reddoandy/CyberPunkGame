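; Default player character that moves, jumps, dashes and shows the battle UI.
; On BattleMap it pulls its team from the game instance by net ID, registers with the game mode, then sets tag, material and shooting/tower-placing component owners.
; Non-tower damage drains health; death locks movement, and Tick respawns it at a PlayerStart once server time passes SpawnTime.
; It also opens character selection UI and has numpad debug damage/kill keys.
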(event Custom|Initialize
  (params (Team :type String))
  (bind _self self)
  (Variables|/Game/Blueprints/MainChar/PlacingResourceTowerSystem.PlacingResourceTowerSystem_C|SetOwnerCharacter (Variables|Default|GetPlacingResourceTowerSystem) _self)
  (Variables|/Game/Blueprints/MainChar/ShootingSystem.ShootingSystem_C|SetOwnerChar (Variables|Default|GetShootingSystem) _self)
  (Variables|Default|SetTeam Team)
  (Utilities|Array|SetArrayElem (Variables|Actor|GetTags) 0 (Utilities|String|StringToName (Variables|Default|GetTeam)) true)
  (Rendering|Material|SetMaterial (Variables|Default|GetSphere) 0 (select (Utilities|Enum|Equal(Enum) (Variables|Default|GetTeam) "Blue") "/Engine/VREditor/LaserPointer/HoverMaterial.HoverMaterial" "/Engine/VREditor/LaserPointer/LaserPointerMaterialInst.LaserPointerMaterialInst")))

(event Custom|DeadServer
  (Default|ChangePlayingState (.AsMy%20Player%20State (Utilities|Casting|CastToMyPlayerState (Variables|GetPlayerState))) "NewEnumerator2")
  (Variables|Default|SetCanMove false)
  (Variables|Default|SetDeadTime (GameState|GetServerWorldTimeSeconds (Game|GetGameState))))

(event Custom|RespawnServer
  (bind _returnvalue (Actor|GetActorOfClass "/Script/Engine.PlayerStart"))
  (Transformation|SetActorLocationAndRotation (Transformation|GetActorLocation _returnvalue) (Transformation|GetActorRotation _returnvalue) false true)
  (Default|ChangePlayingState (.AsMy%20Player%20State (Utilities|Casting|CastToMyPlayerState (Variables|GetPlayerState))) "NewEnumerator0")
  (Variables|Default|SetCanMove true)
  (Variables|Default|SetHealth (Variables|Default|GetMaxHealth)))

(event Custom|Choosecharacter
  (bind _returnvalue (UserInterface|CreateWidget "/Game/Blueprints/UI/PreGameUI/ChooseCharacterUI.ChooseCharacterUI_C"))
  (UserInterface|Viewport|AddtoViewport _returnvalue 0)
  (bind _asplayer_controller (Utilities|Casting|CastToPlayerController (Pawn|GetController)))
  (Input|SetInputModeUIOnly _asplayer_controller 0 "DoNotLock" false))

(event Custom|Dash_Server
  (Character|LaunchCharacter (+ (* (+ (* (Transformation|GetActorRightVector) (.x (stale Input|EnhancedActionEvents|EnhancedInputActionIA_Move ActionValue))) (* (Transformation|GetActorForwardVector) (.y (stale Input|EnhancedActionEvents|EnhancedInputActionIA_Move ActionValue)))) 5e+03) "0.000000,0.000000,10.000000") false false))

(event Input|EnhancedActionEvents|EnhancedInputActionIA_Dash
  (params (ActionValue :type Vector%202D%20Structure) (ElapsedSeconds :type Float%20%28double-precision%29) (TriggeredSeconds :type Float%20%28double-precision%29) (InputAction :type Input%20Action%20Object%20Reference :default "/Game/Blueprints/Input/Actions/IA_Dash.IA_Dash"))
  (Utilities|FlowControl|Sequence :!label _label
    (:then_0
      (Development|PrintString "Dash")
      (CallFunction|DashServer))
    (:then_1
      (Utilities|FlowControl|Delay 5.0)
      (Utilities|FlowControl|DoOnce false ; enters at Reset
        (:Completed
          (goto _label))))))

(event Input|EnhancedActionEvents|EnhancedInputActionIA_Move
  (params (ActionValue :type Vector%202D%20Structure) (ElapsedSeconds :type Float%20%28double-precision%29) (TriggeredSeconds :type Float%20%28double-precision%29) (InputAction :type Input%20Action%20Object%20Reference :default "/Game/Blueprints/Input/Actions/IA_Move.IA_Move"))
  (if (Variables|Default|GetCanMove)
    (Pawn|Input|AddMovementInput (Transformation|GetActorRightVector) (.x ActionValue) false)
    (Pawn|Input|AddMovementInput (Transformation|GetActorForwardVector) (.y ActionValue) false)))

(event Input|EnhancedActionEvents|EnhancedInputActionIA_Look
  (params (ActionValue :type Vector%202D%20Structure) (ElapsedSeconds :type Float%20%28double-precision%29) (TriggeredSeconds :type Float%20%28double-precision%29) (InputAction :type Input%20Action%20Object%20Reference :default "/Game/Blueprints/Input/Actions/IA_Look.IA_Look"))
  (bind _returnvalue (Math|Float|SelectFloat -1.0 1.0 false))
  (Pawn|Input|AddControllerYawInput (* (.x ActionValue) _returnvalue))
  (Pawn|Input|AddControllerPitchInput (* (.y ActionValue) _returnvalue)))

(event Input|EnhancedActionEvents|EnhancedInputActionIA_Jump
  (params (ActionValue :type Boolean) (ElapsedSeconds :type Float%20%28double-precision%29) (TriggeredSeconds :type Float%20%28double-precision%29) (InputAction :type Input%20Action%20Object%20Reference :default "/Game/Blueprints/Input/Actions/IA_Jump.IA_Jump"))
  (:Started
    (if (Variables|Default|GetCanMove)
      (Character|Jump)))
  (:Completed
    (Character|StopJumping)))

(event EventBeginPlay
  (bind _returnvalue (UserInterface|CreateWidget "/Game/Blueprints/UI/BattleUI/BattleUI.BattleUI_C"))
  (UserInterface|Viewport|AddtoViewport _returnvalue 0)
  (bind _returnvalue_2 (Game|GetCurrentLevelName true))
  (if (Utilities|Enum|Equal(Enum) _returnvalue_2 "BattleMap")
    (bind _asbp_my_game_instance (Utilities|Casting|CastToBP_MyGameInstance (Game|GetGameInstance)))
    (bind (_team _index) (Class|MyGameInstance|PullTeamInfo _asbp_my_game_instance (Class|AdvancedSessionsLibrary|UniqueNetIdtoString (Class|AdvancedSessionsLibrary|GetUniqueNetIDfromPlayerState (Variables|GetPlayerState)))))
    (Default|InputPlayerInfo (.AsBP%20Battle%20Game%20Mode (Utilities|Casting|CastToBP_BattleGameMode (Game|GetGameMode))) (.AsPlayer%20Controller (Utilities|Casting|CastToPlayerController (Pawn|GetController))) _team _index)
    (CallFunction|Initialize _team)))

(event Collision|EventActorBeginOverlap
  (params (OtherActor :type Actor%20Object%20Reference)))

(event EventTick
  (params (DeltaSeconds :type Float%20%28single-precision%29))
  (if (Utilities|Enum|Equal(Enum) (Variables|/Game/Blueprints/MainChar/MyPlayerState.MyPlayerState_C|GetPlayingState (.AsMy%20Player%20State (Utilities|Casting|CastToMyPlayerState (Variables|GetPlayerState)))) "NewEnumerator2")
    (if (>= (- (GameState|GetServerWorldTimeSeconds (Game|GetGameState)) (Variables|Default|GetDeadTime)) (Variables|Default|GetSpawnTime))
      (CallFunction|RespawnServer))))

(event Game|Damage|EventAnyDamage
  (params (Damage :type Float%20%28single-precision%29) (DamageType :type Damage%20Type%20Object%20Reference) (InstigatedBy :type Controller%20Object%20Reference) (DamageCauser :type Actor%20Object%20Reference))
  (if (!= DamageType "/Game/Blueprints/System/DamageType/TowerDamage.TowerDamage")
    (Variables|Default|SetHealth (- (Variables|Default|GetHealth) Damage))
    (if (<= (Variables|Default|GetHealth) 0.0)
      (CallFunction|DeadServer))))

(event Input|KeyboardEvents|NumPadZero
  (params (Key :type Key%20Structure :default "None"))
  (:Pressed
    (CallFunction|DeadServer)))

(event Input|KeyboardEvents|NumPadOne
  (params (Key :type Key%20Structure :default "None"))
  (:Pressed
    (Game|Damage|ApplyDamage self 1e+01 0 0)))

(fn ConstructionScript)