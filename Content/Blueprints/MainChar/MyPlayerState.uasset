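; MyPlayerState is a player state Blueprint that holds the player's playing state and three resource totals: Money, Equip and Caculate.
; The ChangePlayingState event overwrites the stored PlayingState with the value passed in.
; The AddResource event switches on a resource type and adds the given value to the matching total, with no clamping or change notification.
; BeginPlay, Tick and the construction script do nothing.
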(event Custom|ChangePlayingState
  (params (State :type PlayingState%20Enum :default "NewEnumerator0"))
  (Variables|Default|SetPlayingState State))

(event Custom|AddResource
  (params (Type :type ResourceType%20Enum :default "NewEnumerator0") (Value :type Integer))
  (switch Utilities|FlowControl|Switch|SwitchonResourceType Type
    (:NewEnumerator0
      (Variables|Default|SetMoney (+ (Variables|Default|GetMoney) Value)))
    (:NewEnumerator1
      (Variables|Default|SetEquip (+ (Variables|Default|GetEquip) Value)))
    (:NewEnumerator2
      (Variables|Default|SetCaculate (+ (Variables|Default|GetCaculate) Value)))))

(event EventBeginPlay)

(event EventTick
  (params (DeltaSeconds :type Float%20%28single-precision%29)))

(fn ConstructionScript)