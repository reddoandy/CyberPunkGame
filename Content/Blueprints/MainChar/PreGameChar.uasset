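; PreGameChar is a placeholder character that handles team setup and character selection before a player gets a battle character.
; On possession in BattleMap, it requests team info from the game instance by NetId, and a completion event passes the result to BP_BattleGameMode and MyPlayerController.
; Separate events show the selection UI, store the chosen class, then spawn it, have the controller possess it and remove the UI.
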(event Custom|EndChoosing
  (Widget|RemovefromParent (stale Custom|Choosecharacter _returnvalue)))

(event Custom|SetChooseChar
  (params (SelectChar :type Pawn%20Class%20Reference))
  (Variables|Default|SetSelectChar SelectChar))

(event Custom|SpawnChooseCharServer
  (params (SpawnTransform :type Transform))
  (bind _returnvalue (Game|SpawnActorfromClass (Variables|Default|GetSelectChar) SpawnTransform "Undefined" "MultiplyWithRoot" 0 0))
  (Pawn|Possess (Pawn|GetController) _returnvalue)
  (CallFunction|EndChoosing))

(event Custom|Choosecharacter
  (bind _returnvalue (UserInterface|CreateWidget "/Game/Blueprints/UI/PreGameUI/ChooseCharacterUI.ChooseCharacterUI_C"))
  (UserInterface|Viewport|AddtoViewport _returnvalue 0)
  (bind _asplayer_controller (Utilities|Casting|CastToPlayerController (Pawn|GetController)))
  (Input|SetInputModeUIOnly _asplayer_controller 0 "DoNotLock" false))

(event Custom|InitClient
  (bind _returnvalue (Game|GetCurrentLevelName true))
  (if (Utilities|Enum|Equal(Enum) _returnvalue "BattleMap")
    (bind _asbp_my_game_instance (Utilities|Casting|CastToBP_MyGameInstance (Game|GetGameInstance)))
    (Class|MyGameInstance|PullTeamInfo _asbp_my_game_instance (Variables|/Game/Blueprints/System/BP_MyGameInstance.BP_MyGameInstance_C|GetNetId _asbp_my_game_instance))))

(event Custom|PullTeamCompelete
  (params (Team :type String) (Index :type Integer))
  (bind _returnvalue (Pawn|GetController))
  (bind _asplayer_controller (Utilities|Casting|CastToPlayerController _returnvalue))
  (Default|InputPlayerInfo (.AsBP%20Battle%20Game%20Mode (Utilities|Casting|CastToBP_BattleGameMode (Game|GetGameMode))) _asplayer_controller Team Index)
  (Default|SetTeam (.AsMy%20Player%20Controller (Utilities|Casting|CastToMyPlayerController _asplayer_controller)) Team))

(event EventBeginPlay)

(event Collision|EventActorBeginOverlap
  (params (OtherActor :type Actor%20Object%20Reference)))

(event EventTick
  (params (DeltaSeconds :type Float%20%28single-precision%29)))

(event EventPossessed
  (params (NewController :type Controller%20Object%20Reference))
  (CallFunction|InitClient))

(fn ConstructionScript)