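; Player controller for the main character that sets up Enhanced Input and holds debug hooks for online identity.
; BeginPlay adds the IMC_MyInputSystem mapping context to the local player's input subsystem.
; CustomEvent queries and prints the login status for the PlayerState's net ID, and SyncUniqueId copies the unique ID to the PlayerState.
; A persistent-auth login and a controller ID print are left unwired.
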(event Custom|CustomEvent
  (bind _loginstatus (Class|AdvancedIdentityLibrary|GetLoginStatus (Class|AdvancedSessionsLibrary|GetUniqueNetIDfromPlayerState (Variables|Default|GetPlayerState)))
    (:OnSuccess
      _)
    (:OnFailure
      _))
  (Development|PrintString (Utilities|String|EnumtoString _loginstatus)))

(event Custom|SyncUniqueId
  (Class|MyPlayerControllerCpp|CopyUniqueIdtoPlayerState)
  (Development|PrintString "Sync"))

(event EventBeginPlay
  (bind _returnvalue (PlayerController|LocalPlayerSubsystems|GetEnhancedInputLocalPlayerSubsystem))
  (Utilities|IsValid _returnvalue
    (:Is%20Valid
      (Input|AddMappingContext _returnvalue "/Game/Blueprints/Input/IMC_MyInputSystem.IMC_MyInputSystem" 0 "(bIgnoreAllPressedKeysUntilRelease=True,bForceImmediately=False,bNotifyUserSettings=False)"))))

(event EventTick
  (params (DeltaSeconds :type Float%20%28single-precision%29)))

(fn ConstructionScript)