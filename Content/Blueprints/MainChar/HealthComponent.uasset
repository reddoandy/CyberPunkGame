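; Health component for the main character that handles timed ExHealth regeneration and ReduceShield decay.
; Server-authority events start a countdown that, after a delay, launches a fast looping timer raising ExHealth in small steps while below MaxExHealth.
; A stop event clears both recovery timers.
; A separate restartable looping timer drains ReduceShield and clears itself once the value is no longer positive.
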(event Custom|SetExHealthRecoverTimer
  (Networking|SwitchHasAuthority
    (:Authority
      (if (Utilities|Time|IsValidTimerHandle (Variables|Default|GetCountdownTimer))
        (Utilities|Time|ClearandInvalidateTimerbyHandle (Variables|Default|GetCountdownTimer)))
      (bind _returnvalue (Utilities|Time|SetTimerbyEvent (delegate Custom|StartExHealthTimer) 5.0))
      (Variables|Default|SetCountdownTimer _returnvalue))))

(event Custom|StartExHealthTimer
  (bind _returnvalue (Utilities|Time|SetTimerbyEvent (delegate Custom|ExHealthRecover) 0.01 true))
  (Variables|Default|SetRecoverTimer _returnvalue))

(event Custom|ExHealthRecover
  (if (< (Variables|Default|GetExHealth) (Variables|Default|GetMaxExHealth))
    (Variables|Default|SetExHealth (+ (Variables|Default|GetExHealth) (/ 1e+01 1e+02)))))

(event Custom|StopExHealthRecover
  (Networking|SwitchHasAuthority
    (:Authority
      (Utilities|Time|ClearandInvalidateTimerbyHandle (Variables|Default|GetRecoverTimer))
      (Utilities|Time|ClearandInvalidateTimerbyHandle (Variables|Default|GetCountdownTimer)))))

(event Custom|SetReduceShieldTimer
  (Networking|SwitchHasAuthority
    (:Authority
      (if (Utilities|Time|IsValidTimerHandle (Variables|Default|GetReduceShieldTimer))
        (Utilities|Time|ClearandInvalidateTimerbyHandle (Variables|Default|GetReduceShieldTimer)))
      (bind _returnvalue (Utilities|Time|SetTimerbyEvent (delegate Custom|RunReduceShield) 0.01 true))
      (Variables|Default|SetReduceShieldTimer _returnvalue))))

(event Custom|RunReduceShield
  (if (> (Variables|Default|GetReduceShield) 0.0)
    (Variables|Default|SetReduceShield (- (Variables|Default|GetReduceShield) (/ 2e+02 1e+02)))
    (else
      (Utilities|Time|ClearandInvalidateTimerbyHandle (Variables|Default|GetReduceShieldTimer)))))

(event EventBeginPlay)

(event EventTick
  (params (DeltaSeconds :type Float%20%28single-precision%29)))