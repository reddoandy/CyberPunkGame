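; Character-side system that lets a player place resource towers while standing inside a Resource Zone.
; Pressing F in a zone switches the player state to PlacingTower and spawns a preview actor, which follows a camera line trace each tick, aligned to the surface normal.
; Left click on a valid spot destroys the preview and calls a server event that spawns the team's tower, registers it with the zone and restores the Normal state.
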(event Custom|PlaceTower_Server
  (params (SpawnTransform :type Transform))
  (bind _ownercharacter (Variables|Default|GetOwnerCharacter))
  (bind _ownercharacter_2 (Variables|Default|GetOwnerCharacter))
  (bind _overlappingactors (Collision|GetOverlappingActors _ownercharacter_2 "/Game/Blueprints/Actors/ResourceCollect/ResourceZone/ResourceZone.ResourceZone_C" :!class /Script/Engine.Actor))
  (bind _playerstate (Variables|/Script/Engine.Pawn|GetPlayerState _ownercharacter))
  (bind _asmy_player_state (Utilities|Casting|CastToMyPlayerState _playerstate))
  (if (Utilities|Array|IsNotEmpty _overlappingactors)
    (bind _array_element (Utilities|Array|ForEachLoopwithBreak _overlappingactors :!label _label)
      (:LoopBody
        (Utilities|IsValid _array_element
          (:Is%20Valid
            (goto _label Break))))
      (:Completed
        (bind _returnvalue (Game|SpawnActorfromClass "/Game/Blueprints/Actors/ResourceCollect/ResourceTower/ResourceTower.ResourceTower_C" SpawnTransform "Undefined" "MultiplyWithRoot" 0 _asmy_player_state (.AsResource%20Zone (Utilities|Casting|CastToResourceZone _array_element)) (Variables|/Game/Blueprints/System/TeamComponent.TeamComponent_C|GetTeam (Variables|/Game/Blueprints/MainChar/DefaultChar.DefaultChar_C|GetTeamComponent _ownercharacter_2)) 0))
        (Utilities|Array|Add (Variables|/Game/Blueprints/Actors/ResourceCollect/ResourceZone/ResourceZone.ResourceZone_C|GetPlacedTowers (.AsResource%20Zone (Utilities|Casting|CastToResourceZone _array_element))) _returnvalue)
        (Utilities|FlowControl|Delay 0.1)
        (Default|ChangePlayingState _asmy_player_state "NewEnumerator0")))))

(event Input|EnhancedActionEvents|EnhancedInputActionIA_LMB
  (params (ActionValue :type Boolean) (ElapsedSeconds :type Float%20%28double-precision%29) (TriggeredSeconds :type Float%20%28double-precision%29) (InputAction :type Input%20Action%20Object%20Reference :default "/Game/Blueprints/Input/Actions/IA_LMB.IA_LMB"))
  (bind _previewtoweractor (Variables|Default|GetPreviewTowerActor))
  (bind _ownercharacter (Variables|Default|GetOwnerCharacter))
  (:Started
    (if (Variables|/Game/Blueprints/MainChar/DefaultChar.DefaultChar_C|GetInitialized _ownercharacter)
      (switch Utilities|FlowControl|Switch|SwitchonPlayingState (Variables|/Game/Blueprints/MainChar/MyPlayerState.MyPlayerState_C|GetPlayingState (.AsMy%20Player%20State (Utilities|Casting|CastToMyPlayerState (Variables|/Script/Engine.Pawn|GetPlayerState _ownercharacter))))
        (:NewEnumerator1
          (Utilities|IsValid _previewtoweractor
            (:Is%20Valid
              (if (not (Variables|/Game/Blueprints/Actors/ResourceCollect/ResourceTower/ResourceTowerPreview.ResourceTowerPreview_C|GetCantPlace _previewtoweractor))
                (Utilities|FlowControl|DoOnce false :!label _label
                  (:Completed
                    (CallFunction|PlaceTowerServer (Transformation|GetActorTransform (Variables|Default|GetPreviewTowerActor)))
                    (Actor|DestroyActor _previewtoweractor)
                    (Utilities|FlowControl|Delay 0.1)
                    (goto _label Reset))))))))
      (else
        (Development|PrintString "Not init")))))

(event EventBeginPlay)

(event EventTick
  (params (DeltaSeconds :type Float%20%28single-precision%29))
  (bind _previewtoweractor (Variables|Default|GetPreviewTowerActor))
  (bind _ownercharacter (Variables|Default|GetOwnerCharacter))
  (bind _previewtoweractor_2 (Variables|Default|GetPreviewTowerActor))
  (bind _camera (Variables|/Game/Blueprints/MainChar/DefaultChar.DefaultChar_C|GetCamera _ownercharacter))
  (bind _returnvalue (Transformation|GetWorldLocation _camera))
  (if (Variables|/Game/Blueprints/MainChar/DefaultChar.DefaultChar_C|GetInitialized (Variables|Default|GetOwnerCharacter))
    (if (Utilities|Enum|Equal(Enum) (Variables|/Game/Blueprints/MainChar/MyPlayerState.MyPlayerState_C|GetPlayingState (.AsMy%20Player%20State (Utilities|Casting|CastToMyPlayerState (Variables|/Script/Engine.Pawn|GetPlayerState _ownercharacter)))) "NewEnumerator1")
      (bind (_outhit _returnvalue_2) (Collision|LineTraceByChannel _returnvalue (+ _returnvalue (* (Math|Vector|GetForwardVector _camera) 2e+03)) "TraceTypeQuery1" false 0 "None"))
      (Utilities|IsValid _previewtoweractor
        (:Is%20Valid
          (if _returnvalue_2
            (Rendering|SetActorHiddenInGame _previewtoweractor false)
            (Variables|Default|SetImpact%20Point (.ImpactPoint (Collision|BreakHitResult _outhit)))
            (Variables|Default|SetImpact%20Normal (.ImpactNormal (Collision|BreakHitResult _outhit)))
            (if (Utilities|IsValid _previewtoweractor_2)
              (Transformation|SetActorLocationAndRotation _previewtoweractor_2 (Variables|Default|GetImpact%20Point) (Math|Rotator|MakeRotfromZ (Variables|Default|GetImpact%20Normal))))
            (else
              (Rendering|SetActorHiddenInGame _previewtoweractor true))))))))

(event Input|KeyboardEvents|F
  (params (Key :type Key%20Structure :default "None"))
  (bind _ownercharacter (Variables|Default|GetOwnerCharacter))
  (bind _playerstate (Variables|/Script/Engine.Pawn|GetPlayerState _ownercharacter))
  (bind _asmy_player_state (Utilities|Casting|CastToMyPlayerState _playerstate))
  (:Pressed
    (if (Variables|/Game/Blueprints/MainChar/DefaultChar.DefaultChar_C|GetInitialized (Variables|Default|GetOwnerCharacter))
      (if (Utilities|Enum|NotEqual(Enum) (Variables|/Game/Blueprints/MainChar/MyPlayerState.MyPlayerState_C|GetPlayingState _asmy_player_state) "NewEnumerator1")
        (if (Utilities|Array|IsNotEmpty (Collision|GetOverlappingActors (Variables|Default|GetOwnerCharacter) "/Game/Blueprints/Actors/ResourceCollect/ResourceZone/ResourceZone.ResourceZone_C" :!class /Script/Engine.Actor))
          (Default|ChangePlayingState _asmy_player_state "NewEnumerator1")
          (bind _returnvalue (Game|SpawnActorfromClass "/Game/Blueprints/Actors/ResourceCollect/ResourceTower/ResourceTowerPreview.ResourceTowerPreview_C" (Math|Transform|MakeTransform (Variables|Default|GetImpact%20Point) (Math|Rotator|MakeRotfromZ (Variables|Default|GetImpact%20Normal)) "1.000000,1.000000,1.000000") "Undefined" "MultiplyWithRoot" 0 _ownercharacter 0))
          (Development|PrintString "Preview")
          (Variables|Default|SetPreviewTowerActor _returnvalue)
          (else
            (Development|PrintString "Not in Resource Zone"))))
      (else
        (Development|PrintString "Not init")))))